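; Manager actor Blueprint that sets up and runs Learning Agents neural-network training.
; On BeginPlay it sets up the interactor, builds a policy on it from the Dat_learn network asset, then passes both to the trainer.
; Every Tick calls RunTraining on the trainer with its training, game, path and critic settings.
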(event `self.ReceiveBeginPlay`
  (`|ExecutionSequence`
    (:`then_0`
      (`LearningAgentsInteractor.SetupInteractor` (`self.BP_inter`)))
    (:`then_1`
      (`LearningAgentsPolicy.SetupPolicy` (`self.BP_poly`) (`self.BP_inter`) (`self.Policy Settings`) "/Game/LearnAgent/Dat_learn.Dat_learn"))
    (:`then_2`
      (`LearningAgentsTrainer.SetupTrainer` (`self.BP_train`) (`self.BP_inter`) (`self.BP_poly`) null (`self.Trainer Settings`)))))

(event `self.ReceiveTick`
  (params (DeltaSeconds :type "Float (single-precision)"))
  (`LearningAgentsTrainer.RunTraining` (`self.BP_train`) (`self.Trainer Training Settings`) (`self.Trainer Game Settings`) (`self.Trainer Path Settings`) (`self.Critic Settings`) true true true))

(fn `UserConstructionScript`)